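; Coin pickup actor that adds one to the player's currency when touched.
; On overlap it passes the other actor's name to CheckPlayerHit, then casts that actor to Jussi and increments its Currency.
; It then plays the CoinCollected 2D sound and calls the CoinPickedED dispatcher.
; The coin does not destroy or hide itself in this graph.
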(event `self.ReceiveActorBeginOverlap`
  (params (OtherActor :type "Actor Object Reference"))
  (bind _result (`self.Check Player Hit` (`KismetSystemLibrary.GetObjectName` OtherActor)))
  (if _result
    (bind _asjussi (cast `/Game/Characters/Player/Jussi` OtherActor))
    (bind _result_2 (`/Engine/EditorBlueprintResources/StandardMacros.IncrementInt` (`/Game/Characters/Player/Jussi.Currency` _asjussi))
      (:`  `
        (set `/Game/Characters/Player/Jussi.Currency` _result_2 _asjussi)
        (`GameplayStatics.PlaySound2D` "/Game/SoundEffects/CoinCollected.CoinCollected" 1.0 1.0 0.0 null null)
        (`self.Coin Picked ED`)))))

(event `self.ReceiveTick`
  (params (DeltaSeconds :type "Float (single-precision)")))

(fn `UserConstructionScript`
  (`parent.UserConstructionScript`))