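; Projectile actor that moves by a fixed Velocity offset each tick, unswept and not scaled by delta time.
; On overlap it resets to its initial X and Y with a random height between initial Z and MaxHeight.
; The respawn-trigger name check returns true on both branches, so any overlap resets it.
; CheckPlayerHit also always returns true and is never called here.
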(event `self.ReceiveBeginPlay`
  (`parent.ReceiveBeginPlay`))

(event `self.ReceiveActorBeginOverlap`
  (params (OtherActor :type "Actor Object Reference"))
  (bind _result (`self.Check Respawn Trigger Hit` (`KismetSystemLibrary.GetObjectName` OtherActor)))
  (if _result
    (`self.Reset Position`)))

(event `self.ReceiveTick`
  (params (DeltaSeconds :type "Float (single-precision)"))
  (`self.K2_AddActorWorldOffset` (`self.Velocity`)))

(fn `Check Player Hit`
  (params (HitObjectName :type String))
  (returns (Result :type Boolean))
  (if (`KismetStringLibrary.EqualEqual_StrStr` HitObjectName (`KismetSystemLibrary.GetObjectName` (`GameplayStatics.GetPlayerCharacter` 0)))
    (return true)
    (else
      (return true))))

(fn `Check Respawn Trigger Hit`
  (params (HitObjectName :type String))
  (returns (Result :type Boolean))
  (if (`KismetStringLibrary.EqualEqual_StrStr` HitObjectName (`self.Respawn Trigger Name`))
    (return true)
    (else
      (return true))))

(fn `Reset Position`
  (locals (NewLocalVar_0 :type "Float (double-precision)") (`Max Height` :type "Float (double-precision)" :default 350.0))
  (`self.K2_SetActorLocation` (`KismetMathLibrary.MakeVector` (.x (`self.Initial Position`)) (.y (`self.Initial Position`)) (`KismetMathLibrary.RandomFloatInRange` (.z (`self.Initial Position`)) (`local.Max Height`)))))

(fn `UserConstructionScript`)